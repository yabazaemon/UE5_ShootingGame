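; BP_MainCamera turns the player character to face the mouse cursor, though its graphs contain no camera movement logic.
; Each Tick deprojects the cursor to a world ray and intersects it with the world Z=0 plane, without a trace.
; It applies only the look-at yaw toward that point, zeroing pitch and roll and teleporting physics.
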(event `self.ReceiveTick`
  (params (DeltaSeconds :type "Float (single-precision)"))
  (bind (_worldlocation _worlddirection _returnvalue) (`PlayerController.DeprojectMousePositionToWorld` (`GameplayStatics.GetPlayerController` 0)))
  (if _returnvalue
    (`self.K2_SetActorRotation` (`GameplayStatics.GetPlayerCharacter` 0) (`KismetMathLibrary.MakeRotator` 0.0 0.0 (.yaw (`KismetMathLibrary.FindLookAtRotation` (`self.K2_GetActorLocation` (`GameplayStatics.GetPlayerCharacter` 0)) (+ _worldlocation (* _worlddirection (/ (* (.z _worldlocation) -1.0) (.z _worlddirection))))))) true)))

(fn `UserConstructionScript`)