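; BP_PlayerBullet is the player's bullet, gaining energy on hits and able to be absorbed back by the player.
; On spawn it sets a lifespan and, if the player is not charging, resets damage and energy to normal-shot values.
; Hits add energy up to a count limit, then multiply it, before calling HandleHitAndApplyDamage.
; Overlapping an absorbing player adds its energy to BP_PlayerState and destroys the bullet.
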(event `self.ReceiveBeginPlay`
  (`parent.ReceiveBeginPlay`)
  (bind _asbp_player (cast `/Game/BluePrint/BP_Player` (`GameplayStatics.GetPlayerPawn` 0)))
  (if (`/Game/BluePrint/BP_Player.Charging` _asbp_player)
    (`self.SetLifeSpan` (`self.In Lifespan`))
    (else
      (bind _output_get (set `self.Base Damage` 1.0))
      (set `self.BulletEnergy` (`KismetMathLibrary.FTrunc` _output_get))
      (`KismetSystemLibrary.PrintString` "NomalShot")
      (`self.SetLifeSpan` (`self.In Lifespan`)))))

(event `self.ReceiveActorBeginOverlap`
  (params (OtherActor :type "Actor Object Reference"))
  (`parent.ReceiveActorBeginOverlap` OtherActor)
  (bind _asbp_player (cast `/Game/BluePrint/BP_Player` OtherActor))
  (if (`/Game/BluePrint/BP_Player.Absorbing` _asbp_player)
    (bind _asbp_player_state (cast `/Game/BluePrint/BP_PlayerState` (`GameplayStatics.GetPlayerState` 0)))
    (set `/Game/BluePrint/BP_PlayerState.Player Energy` (+ (`/Game/BluePrint/BP_PlayerState.Player Energy` _asbp_player_state) (`self.BulletEnergy`)) _asbp_player_state)
    (`self.K2_DestroyActor`)))

(event `self.ReceiveHit`
  (params (MyComp :type "PrimitiveComponent Object Reference") (Other :type "Actor Object Reference") (OtherComp :type "PrimitiveComponent Object Reference") (bSelfMoved :type Boolean) (HitLocation :type "Vector Structure") (HitNormal :type "Vector Structure") (NormalImpulse :type "Vector Structure") (Hit :type "HitResult Structure (by ref)"))
  (if (< (stale _counter) (`self.ReasonDabUp`))
    (bind _counter (`/Engine/EditorBlueprintResources/StandardMacros.Do N` (`self.ReasonDabUp`))
      (:`Exit`
        (bind _output_get (set `self.BulletEnergy` (+ (`self.BulletEnergy`) 1)))
        (`KismetSystemLibrary.PrintString` (`KismetStringLibrary.Conv_IntToString` _output_get))))
    (else
      (bind _output_get_2 (set `self.BulletEnergy` (* (`self.BulletEnergy`) (`self.EnergyMultiPer`))))
      (`KismetSystemLibrary.PrintString` (`KismetStringLibrary.Conv_IntToString` _output_get_2))))
  (`self.HandleHitAndApplyDamage` null Other bSelfMoved HitLocation HitNormal NormalImpulse Hit))

(fn `UserConstructionScript`
  (`parent.UserConstructionScript`))