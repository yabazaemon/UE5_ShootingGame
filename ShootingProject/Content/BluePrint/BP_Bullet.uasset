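; BP_Bullet is a bullet actor that holds itself at a constant height.
; BeginPlay stores its starting Z, and every Tick resets the actor to that Z while keeping its current X and Y, without sweep or teleport.
; The graph contains no propulsion or hit logic: the overlap event is an unused placeholder and the construction script only calls its parent.
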(event `self.ReceiveBeginPlay`
  (set `self.Actor InisialZ` (.z (`self.K2_GetActorLocation`))))

(event `self.ReceiveTick`
  (params (DeltaSeconds :type "Float (single-precision)"))
  (`self.K2_SetActorLocation` (`KismetMathLibrary.MakeVector` (.x (`self.K2_GetActorLocation`)) (.y (`self.K2_GetActorLocation`)) (`self.Actor InisialZ`))))

(fn `UserConstructionScript`
  (`parent.UserConstructionScript`))