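; Player pawn Blueprint with movement along world axes, a normal shot, a charge shot and an absorb action, driven by Enhanced Input.
; Normal shots spawn BP_PlayerBullet at ShootPoint unless charged; the charge shot only prints its time and resets.
; Tick uses a collapsed graph to toggle absorb collision and mesh from the Absorbing flag.
; The charge timer hangs off Tick's absorbing branch, although charging can only start while not absorbing.
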(event `self.ReceiveTick`
  (params (DeltaSeconds :type "Float (single-precision)"))
  (if (`self.Absorbing`)
    (`PrimitiveComponent.SetCollisionEnabled` (`self.AbsorbCollision`) "QueryAndPhysics")
    (`SceneComponent.SetVisibility` (`self.Absorb Mesh`) true false)
    (else
      (`PrimitiveComponent.SetCollisionEnabled` (`self.AbsorbCollision`) "NoCollision")
      (`PrimitiveComponent.SetCollisionEnabled` (`self.CapsuleComponent`) "QueryAndPhysics")
      (`SceneComponent.SetVisibility` (`self.Absorb Mesh`) false false)
      (if (`self.ButtonPressedCharging`)
        (bind _output_get (set `self.ChragingTime` (+ DeltaSeconds (`self.ChragingTime`))))
        (if (>= _output_get (`self.Charging Reason`))
          (set `self.Charging` true))))))

(event `Normal Shot`
  ;[0.9723 0.2825 1] Normal Shot
  (`KismetSystemLibrary.PrintString` "Shoot")
  (`|SpawnActorFromClass` "/Game/BluePrint/BP_PlayerBullet.BP_PlayerBullet_C" (`SceneComponent.GetSocketTransform` (`self.Aroow`) "ShootPoint" "RTS_World") "Undefined" "MultiplyWithRoot" null 1.0 null))

(event `ChargingShot`
  (`KismetSystemLibrary.PrintString` (`KismetStringLibrary.Conv_DoubleToString` (`self.ChragingTime`)))
  (set `self.Charging` false))

(event `EnhancedInput|/Game/Inputs/IA_Shoot`
  (params (ActionValue :type Boolean) (ElapsedSeconds :type "Float (double-precision)") (TriggeredSeconds :type "Float (double-precision)") (InputAction :type "InputAction Object Reference" :default "/Game/Inputs/IA_Shoot.IA_Shoot"))
  (:`Triggered`
    (if (not (`self.Charging`))
      (`self.Normal Shot`))))

(event `EnhancedInput|/Game/Inputs/IA_ChargeShot`
  (params (ActionValue :type Boolean) (ElapsedSeconds :type "Float (double-precision)") (TriggeredSeconds :type "Float (double-precision)") (InputAction :type "InputAction Object Reference" :default "/Game/Inputs/IA_ChargeShot.IA_ChargeShot"))
  (:`Started`
    (if (not (`self.Absorbing`))
      (set `self.ButtonPressedCharging` true)
      (set `self.ChragingTime` 0.0)
      (set `self.Charging` false)))
  (:`Completed`
    (set `self.ButtonPressedCharging` false)
    (if (`self.Charging`)
      (`self.ChargingShot`))))

(event `EnhancedInput|/Game/Inputs/IA_Absorb`
  (params (ActionValue :type Boolean) (ElapsedSeconds :type "Float (double-precision)") (TriggeredSeconds :type "Float (double-precision)") (InputAction :type "InputAction Object Reference" :default "/Game/Inputs/IA_Absorb.IA_Absorb"))
  (:`Triggered`
    (set `self.Absorbing` true)
    (`KismetSystemLibrary.PrintString` "Absorb"))
  (:`Canceled`
    (set `self.Absorbing` false :!label _label)
    (`KismetSystemLibrary.PrintString` "FinAbsorb"))
  (:`Completed`
    (goto _label)))

(event `EnhancedInput|/Game/Inputs/IA_Move`
  (params (ActionValue :type "Vector2D Structure") (ElapsedSeconds :type "Float (double-precision)") (TriggeredSeconds :type "Float (double-precision)") (InputAction :type "InputAction Object Reference" :default "/Game/Inputs/IA_Move.IA_Move"))
  (bind (_x _y) (`KismetMathLibrary.BreakVector2D` ActionValue))
  (:`Triggered`
    (`self.AddMovementInput` (1.0 0.0 0.0) _y)
    (`self.AddMovementInput` (0.0 1.0 0.0) _x)))

(fn `UserConstructionScript`
  (`parent.UserConstructionScript`))