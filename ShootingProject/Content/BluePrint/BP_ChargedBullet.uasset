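; BP_ChargedBullet is a charged-shot projectile that passes its hit events to HandleHitAndApplyDamage to apply damage.
; On BeginPlay it runs the parent logic, then prints the player pawn's ChargeBulletEnergy from BP_Player for debugging.
; Lifespan setup, a timeline-driven lifetime countdown ending in destruction, and bullet-energy increment and multiplier logic remain in the graph but are never triggered.
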(event `self.ReceiveBeginPlay`
  (`parent.ReceiveBeginPlay`)
  (bind _asbp_player (cast `/Game/BluePrint/BP_Player` (`GameplayStatics.GetPlayerPawn` 0)))
  (`KismetSystemLibrary.PrintString` "ChargeShot" true true (struct :`R` 0.065688 :`G` 0.07899 :`B` 1.0 :`A` 1.0))
  (`KismetSystemLibrary.PrintString` (`KismetStringLibrary.Conv_DoubleToString` (`/Game/BluePrint/BP_Player.ChargeBulletEnergy` _asbp_player)) true true (struct :`R` 0.065688 :`G` 0.07899 :`B` 1.0 :`A` 1.0)))

(event `self.ReceiveHit`
  (params (MyComp :type "PrimitiveComponent Object Reference") (Other :type "Actor Object Reference") (OtherComp :type "PrimitiveComponent Object Reference") (bSelfMoved :type Boolean) (HitLocation :type "Vector Structure") (HitNormal :type "Vector Structure") (NormalImpulse :type "Vector Structure") (Hit :type "HitResult Structure (by ref)"))
  (`self.HandleHitAndApplyDamage` null Other bSelfMoved HitLocation HitNormal NormalImpulse Hit))

(fn `InitializeLifeSettings`
  (params (InitialLifeSpan :type "Float (double-precision)")))

(fn `UserConstructionScript`
  (`parent.UserConstructionScript`))